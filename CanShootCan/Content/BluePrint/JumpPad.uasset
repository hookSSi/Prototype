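; JumpPad is an actor that launches an overlapping CharacterBP straight up with a fixed velocity and handles a jump pad sound.
; The overlap event launches the character and sets an IsActive flag.
; While the flag is set, Tick passes the sound and the character's CanJump result to its SoundEffectManager, whose return value updates IsActive.
; Tick reuses the overlap event's OtherActor and logs a failure if the cast fails.
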(event `self.ReceiveActorBeginOverlap`
  (params (OtherActor :type "Actor Object Reference"))
  ;[1 1 1] Jumping Power
  (bind _ascharacter_bp (cast `/Game/Character/CharacterBP` OtherActor))
  (`Character.LaunchCharacter` _ascharacter_bp (0.0 0.0 1000.0) false false)
  (set `self.bIsActive` true))

(event `self.ReceiveTick`
  (params (DeltaSeconds :type "Float (single-precision)"))
  ;[1 1 1] Jumping Pad Sound
  (if (`self.bIsActive`)
    (bind _ascharacter_bp (cast `/Game/Character/CharacterBP` (stale `self.ReceiveActorBeginOverlap` OtherActor))
      (:`then`
        (bind _isplaying (`/Game/Character/CharacterBP.SoundEffectManager` _ascharacter_bp "/Game/Audio/JumpingPadSound.JumpingPadSound" (`Character.CanJump` _ascharacter_bp)))
        (set `self.bIsActive` _isplaying))
      (:`CastFailed`
        (`VisualLoggerKismetLibrary.LogText` "Failed")))))

(fn `UserConstructionScript`)